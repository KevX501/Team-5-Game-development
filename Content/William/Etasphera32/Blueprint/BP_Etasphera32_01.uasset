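; BP_Etasphera32_01 assembles the Etasphera32 figure from separate skeletal mesh components for the body, arms, hands, individual finger segments and legs.
; The construction script sets Mesh as the master pose component for every listed part, so the pieces follow its bone pose as one modular body.
; The file shows only this pose linkage, with no gameplay logic.
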(fn `UserConstructionScript`
  (`SkinnedMeshComponent.SetLeaderPoseComponent` (`self.SK_Etasphera32_Arm_thumb_01_l`) (`self.Mesh`) false)
  (`SkinnedMeshComponent.SetLeaderPoseComponent` (`self.SK_Etasphera32_Arm_hand_r`) (`self.Mesh`) false)
  (`SkinnedMeshComponent.SetLeaderPoseComponent` (`self.SK_Etasphera32_Arm_index_01_l`) (`self.Mesh`) false)
  (`SkinnedMeshComponent.SetLeaderPoseComponent` (`self.SK_Etasphera32_Arm_index_01_r`) (`self.Mesh`) false)
  (`SkinnedMeshComponent.SetLeaderPoseComponent` (`self.SK_Etasphera32_Arm_index_02_l`) (`self.Mesh`) false)
  (`SkinnedMeshComponent.SetLeaderPoseComponent` (`self.SK_Etasphera32_Arm_index_02_r`) (`self.Mesh`) false)
  (`SkinnedMeshComponent.SetLeaderPoseComponent` (`self.SK_Etasphera32_Arm_index_03_l`) (`self.Mesh`) false)
  (`SkinnedMeshComponent.SetLeaderPoseComponent` (`self.SK_Etasphera32_Arm_index_03_r`) (`self.Mesh`) false)
  (`SkinnedMeshComponent.SetLeaderPoseComponent` (`self.SK_Etasphera32_Arm_lowerarm_l`) (`self.Mesh`) false)
  (`SkinnedMeshComponent.SetLeaderPoseComponent` (`self.SK_Etasphera32_Arm_lowerarm_r`) (`self.Mesh`) false)
  (`SkinnedMeshComponent.SetLeaderPoseComponent` (`self.SK_Etasphera32_Arm_middle_01_l`) (`self.Mesh`) false)
  (`SkinnedMeshComponent.SetLeaderPoseComponent` (`self.SK_Etasphera32_Arm_middle_01_r`) (`self.Mesh`) false)
  (`SkinnedMeshComponent.SetLeaderPoseComponent` (`self.SK_Etasphera32_Arm_middle_02_l`) (`self.Mesh`) false)
  (`SkinnedMeshComponent.SetLeaderPoseComponent` (`self.SK_Etasphera32_Arm_middle_02_r`) (`self.Mesh`) false)
  (`SkinnedMeshComponent.SetLeaderPoseComponent` (`self.SK_Etasphera32_Arm_middle_03_l`) (`self.Mesh`) false)
  (`SkinnedMeshComponent.SetLeaderPoseComponent` (`self.SK_Etasphera32_Arm_middle_03_r`) (`self.Mesh`) false)
  (`SkinnedMeshComponent.SetLeaderPoseComponent` (`self.SK_Etasphera32_Arm_ring_01_l`) (`self.Mesh`) false)
  (`SkinnedMeshComponent.SetLeaderPoseComponent` (`self.SK_Etasphera32_Arm_ring_01_r`) (`self.Mesh`) false)
  (`SkinnedMeshComponent.SetLeaderPoseComponent` (`self.SK_Etasphera32_Arm_ring_02_l`) (`self.Mesh`) false)
  (`SkinnedMeshComponent.SetLeaderPoseComponent` (`self.SK_Etasphera32_Arm_ring_02_r`) (`self.Mesh`) false)
  (`SkinnedMeshComponent.SetLeaderPoseComponent` (`self.SK_Etasphera32_Arm_ring_03_l`) (`self.Mesh`) false)
  (`SkinnedMeshComponent.SetLeaderPoseComponent` (`self.SK_Etasphera32_Arm_ring_03_r`) (`self.Mesh`) false)
  (`SkinnedMeshComponent.SetLeaderPoseComponent` (`self.SK_Etasphera32_Arm_hand_l`) (`self.Mesh`) false)
  (`SkinnedMeshComponent.SetLeaderPoseComponent` (`self.SK_Etasphera32_Arm_thumb_01_r`) (`self.Mesh`) false)
  (`SkinnedMeshComponent.SetLeaderPoseComponent` (`self.SK_Etasphera32_Arm_thumb_02_l`) (`self.Mesh`) false)
  (`SkinnedMeshComponent.SetLeaderPoseComponent` (`self.SK_Etasphera32_Arm_thumb_02_r`) (`self.Mesh`) false)
  (`SkinnedMeshComponent.SetLeaderPoseComponent` (`self.SK_Etasphera32_Arm_thumb_03_l`) (`self.Mesh`) false)
  (`SkinnedMeshComponent.SetLeaderPoseComponent` (`self.SK_Etasphera32_Arm_thumb_03_r`) (`self.Mesh`) false)
  (`SkinnedMeshComponent.SetLeaderPoseComponent` (`self.SK_Etasphera32_Arm_upperarm_l`) (`self.Mesh`) false)
  (`SkinnedMeshComponent.SetLeaderPoseComponent` (`self.SK_Etasphera32_Arm_upperarm_r`) (`self.Mesh`) false)
  (`SkinnedMeshComponent.SetLeaderPoseComponent` (`self.SK_Etasphera32_Body_Arm_01_l`) (`self.Mesh`) false)
  (`SkinnedMeshComponent.SetLeaderPoseComponent` (`self.SK_Etasphera32_Body_Arm_01_r`) (`self.Mesh`) false)
  (`SkinnedMeshComponent.SetLeaderPoseComponent` (`self.SK_Etasphera32_Body_Arm_02_l`) (`self.Mesh`) false)
  (`SkinnedMeshComponent.SetLeaderPoseComponent` (`self.SK_Etasphera32_Body_Arm_02_r`) (`self.Mesh`) false)
  (`SkinnedMeshComponent.SetLeaderPoseComponent` (`self.SK_Etasphera32_Body_Arm_03_l`) (`self.Mesh`) false)
  (`SkinnedMeshComponent.SetLeaderPoseComponent` (`self.SK_Etasphera32_Body_Arm_03_r`) (`self.Mesh`) false)
  (`SkinnedMeshComponent.SetLeaderPoseComponent` (`self.SK_Etasphera32_Body_Hips`) (`self.Mesh`) false)
  (`SkinnedMeshComponent.SetLeaderPoseComponent` (`self.SK_Etasphera32_Body_Spine_1`) (`self.Mesh`) false)
  (`SkinnedMeshComponent.SetLeaderPoseComponent` (`self.SK_Etasphera32_Body_Spine_2`) (`self.Mesh`) false)
  (`SkinnedMeshComponent.SetLeaderPoseComponent` (`self.SK_Etasphera32_Leg_calf_l`) (`self.Mesh`) false)
  (`SkinnedMeshComponent.SetLeaderPoseComponent` (`self.SK_Etasphera32_Leg_calf_r`) (`self.Mesh`) false)
  (`SkinnedMeshComponent.SetLeaderPoseComponent` (`self.SK_Etasphera32_Leg_foot_l`) (`self.Mesh`) false)
  (`SkinnedMeshComponent.SetLeaderPoseComponent` (`self.SK_Etasphera32_Leg_foot_r`) (`self.Mesh`) false)
  (`SkinnedMeshComponent.SetLeaderPoseComponent` (`self.SK_Etasphera32_Leg_thigh_l`) (`self.Mesh`) false)
  (`SkinnedMeshComponent.SetLeaderPoseComponent` (`self.SK_Etasphera32_Leg_thigh_r`) (`self.Mesh`) false))