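; BP_TimePickup is a pickup that changes the countdown timer stored in T5GameInstance when the player character overlaps it.
; The RefreshOrRefill flag selects the mode: when true it adds TimerRefill to SecondsLeft and destroys itself.
; When false it resets SecondsLeft to a hardcoded value and stays in the world, so it can trigger again.
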(event `self.ReceiveActorBeginOverlap`
  (params (OtherActor :type "Actor Object Reference"))
  (if (== OtherActor (`GameplayStatics.GetPlayerCharacter` 0))
    (if (`self.RefreshOrRefill?`)
      ;[1 1 1] Refill time
      (bind _ast5game_instance (cast `/Game/Brent/T5GameInstance` (`GameplayStatics.GetGameInstance`)))
      (set `/Game/Brent/T5GameInstance.SecondsLeft` (+ (`/Game/Brent/T5GameInstance.SecondsLeft` _ast5game_instance) (`self.TimerRefill`)) _ast5game_instance)
      (`self.K2_DestroyActor`)
      (else
        ;[1 1 1] Refresh timer
        (bind _ast5game_instance_2 (cast `/Game/Brent/T5GameInstance` (`GameplayStatics.GetGameInstance`)))
        (set `/Game/Brent/T5GameInstance.SecondsLeft` 60 _ast5game_instance_2)))))

(fn `UserConstructionScript`)